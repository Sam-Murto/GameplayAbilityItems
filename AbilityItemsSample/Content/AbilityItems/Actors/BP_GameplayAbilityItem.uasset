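; BP_GameplayAbilityItem is an item actor that grants an ItemAbility to its ItemAbilitySystemComponent on BeginPlay.
; An optional self-activation mode, normally left off, demonstrates the item without a character by sending AbilityItem.Use gameplay events to itself.
; A looping timer sends Start followed by a delayed Release, while Tick sends Trigger every frame.
; The SelfActivated macro gates all three sends on the SelfActivated flag.
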(event Custom|SelfActivateStart
  ;[1 1 1] Self Activation Events - Intended to show funcitonality without a character but normally should not be turned on
  (Utilities|SelfActivated
    (:SelfActivated
      (Ability|SendGameplayEventtoActor self "(TagName=\"AbilityItem.Use.Start\")")
      (Utilities|FlowControl|Delay 0.25)
      (CallFunction|SelfActivateRelease))))

(event Custom|SelfActivateTrigger
  ;[1 1 1] Self Activation Events - Intended to show funcitonality without a character but normally should not be turned on
  (Utilities|SelfActivated
    (:SelfActivated
      (Ability|SendGameplayEventtoActor self "(TagName=\"AbilityItem.Use.Trigger\")"))))

(event Custom|SelfActivateRelease
  ;[1 1 1] Self Activation Events - Intended to show funcitonality without a character but normally should not be turned on
  (Utilities|SelfActivated
    (:SelfActivated
      (Ability|SendGameplayEventtoActor self "(TagName=\"AbilityItem.Use.Release\")"))))

(event EventBeginPlay
  (GameplayAbilities|GiveAbility (Variables|Default|GetItemAbilitySystemComponent) (Variables|AbilityItems|GetItemAbility) 0 -1)
  (Utilities|Time|SetTimerbyEvent (delegate Custom|SelfActivateStart) 1.0 true))

(event EventTick
  (params (DeltaSeconds :type Float%20%28single-precision%29))
  (CallFunction|SelfActivateTrigger))

(fn ConstructionScript)